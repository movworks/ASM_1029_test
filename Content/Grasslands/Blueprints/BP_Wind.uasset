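; BP_Wind is a wind controller that drives foliage and grass materials plus falling-leaf effects.
; Tick advances time values and writes wind, sun, mask and color settings to two Material Parameter Collections, plus player position for trample once CharacterRef is assigned.
; It also feeds wind direction to FX_Falling_Leaves Niagara actors found at BeginPlay.
; An optional one-shot demo chains timelines through direction, mask, color, calm and gust changes; the editor-simulation path is unwired.
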(event `self.ReceiveBeginPlay`
  ;[1 1 1] Event Begin Play
  ;[1 1 1] Set Not Editor
  (set `self.NotEditor?` true)
  ;[1 0.8941 0.1451] Set Niagra VFX Falling Leaves Array
  (bind _outactors (`GameplayStatics.GetAllActorsOfClass` "/Script/Niagara.NiagaraActor"))
  (set `self.VFX_Array` _outactors)
  (`/Engine/EditorBlueprintResources/StandardMacros.IsValid` (`|GetArrayItem` (`self.VFX_Array`))
    (:`Is Valid`
      (`KismetArrayLibrary.Array_Clear` (`self.Niagra_VFX_Array_Ref`))
      (for _array_element (`self.VFX_Array`)
        (set `self.Array_Element_Ref` _array_element)
        (if (== (`KismetSystemLibrary.GetDisplayName` (`self.Array_Element_Ref`)) "FX_Falling_Leaves")
          (`KismetArrayLibrary.Array_Add` (`self.Niagra_VFX_Array_Ref`) (`self.Array_Element_Ref`)))))))

(event `self.ReceiveTick`
  (params (DeltaSeconds :type "Float (single-precision)"))
  (bind _time_add_value_ref (`self.Time_Add_Value_Ref`))
  (bind _wind_power_max_ref (`self.Wind_Power_Max_Ref`))
  (bind _wind_power_min_ref (`self.Wind_Power_Min_Ref`))
  (bind _time_add_value_ref_2 (`self.Time_Add_Value_Ref`))
  (bind _wind_power_max_ref_2 (`self.Wind_Power_Max_Ref`))
  (bind _mask_power_ref (`self.Mask_Power_Ref`))
  (bind (_x _y _z) (`KismetMathLibrary.BreakVector3f` (`self.K2_GetActorLocation` (`self.Character_Ref`))))
  ;[1 1 1] Event Tick - Increase Time Value
  (if (`self.TimeOff?`)
    _
    (elif (`self.NotEditor?`)
      (set `self.Current_Speed_Ref` DeltaSeconds)
      (set `self.Time_Value` (+ (`self.Time_Value`) (`self.Time_Add_Value`)))
      (set `self.Mask_Time` (+ (`self.Mask_Time`) (`self.Mask_Time_Add_Value`)))
      ;[0.2854 1 0.2935] Set Material Scalar Parameters - Wind
      (`KismetMaterialLibrary.SetScalarParameterValue` "/Game/Grasslands/Materials/Grass/MP_Foliage_Parameters.MP_Foliage_Parameters" "BP_Driven_Time" (`self.Time_Value`))
      (`KismetMaterialLibrary.SetScalarParameterValue` "/Game/Grasslands/Materials/Grass/MP_Foliage_Parameters.MP_Foliage_Parameters" "Wind_Power_Max" (`self.Wind_Power_Max`))
      (`KismetMaterialLibrary.SetScalarParameterValue` "/Game/Grasslands/Materials/Grass/MP_Foliage_Parameters.MP_Foliage_Parameters" "Previous_Wind_Drection" (`self.Previous_Wind_Direction`))
      (`KismetMaterialLibrary.SetScalarParameterValue` "/Game/Grasslands/Materials/Grass/MP_Foliage_Parameters.MP_Foliage_Parameters" "Noise_Swap_Value" (`self.Noise_Swap_Value`))
      (`KismetMaterialLibrary.SetScalarParameterValue` "/Game/Grasslands/Materials/Grass/MP_Foliage_Parameters.MP_Foliage_Parameters" "Wind_Power_Min" (`self.Wind_Power_Min`))
      (`KismetMaterialLibrary.SetScalarParameterValue` "/Game/Grasslands/Materials/Grass/MP_Foliage_Parameters.MP_Foliage_Parameters" "Global_Wind_Direction" (`self.Global_Wind_Direction`))
      (`KismetMaterialLibrary.SetScalarParameterValue` "/Game/Grasslands/Materials/Grass/MP_Foliage_Parameters.MP_Foliage_Parameters" "Calm_Wind" (`self.Calm_Wind`))
      (`KismetMaterialLibrary.SetVectorParameterValue` "/Game/Grasslands/Materials/Grass/MP_Foliage_Parameters.MP_Foliage_Parameters" "Sun_Direction" (`self.Sun_Direction`))
      ;[1 0.3804 0.8745] Set Material Scalar Parameters - Mask
      (`KismetMaterialLibrary.SetScalarParameterValue` "/Game/Grasslands/Materials/Landscape/MP_Grass_Mask.MP_Grass_Mask" "Time" (`self.Mask_Time`))
      (`KismetMaterialLibrary.SetScalarParameterValue` "/Game/Grasslands/Materials/Landscape/MP_Grass_Mask.MP_Grass_Mask" "Speed_XY" (`self.Mask_Speed_XY`))
      (`KismetMaterialLibrary.SetScalarParameterValue` "/Game/Grasslands/Materials/Landscape/MP_Grass_Mask.MP_Grass_Mask" "Speed_Z" (`self.Mask_Speed_Z`))
      (`KismetMaterialLibrary.SetScalarParameterValue` "/Game/Grasslands/Materials/Landscape/MP_Grass_Mask.MP_Grass_Mask" "Tiling" (`self.Mask_Tiling`))
      (`KismetMaterialLibrary.SetScalarParameterValue` "/Game/Grasslands/Materials/Landscape/MP_Grass_Mask.MP_Grass_Mask" "Mask_Power" (`self.Mask_Power`))
      (`KismetMaterialLibrary.SetScalarParameterValue` "/Game/Grasslands/Materials/Landscape/MP_Grass_Mask.MP_Grass_Mask" "Grass_Mask_Wind_Direction" (`self.Grass_Mask_Wind_Direction`))
      ;[0.3373 0.4118 1] Set Material Scalar Parameters - Color
      (`KismetMaterialLibrary.SetVectorParameterValue` "/Game/Grasslands/Materials/Grass/MP_Foliage_Parameters.MP_Foliage_Parameters" "Color_Lower" (`self.Color_Lower`))
      (`KismetMaterialLibrary.SetVectorParameterValue` "/Game/Grasslands/Materials/Grass/MP_Foliage_Parameters.MP_Foliage_Parameters" "Color_Upper" (`self.Color_Upper`))
      (`KismetMaterialLibrary.SetVectorParameterValue` "/Game/Grasslands/Materials/Grass/MP_Foliage_Parameters.MP_Foliage_Parameters" "Color_Noise" (`self.Color_Noise`))
      ;[1 1 1] Set Player Position for Trample
      (`/Engine/EditorBlueprintResources/StandardMacros.IsValid` (`self.Character_Ref`)
        (:`Is Valid`
          _)
        (:`Is Not Valid`
          ;;[1 0 0.02983] Set "Character Ref" to a reference to your Character to enable Trample
          (set `self.Character_Ref` null)))
      (`/Engine/EditorBlueprintResources/StandardMacros.IsValid` (`self.Character_Ref`)
        (:`Is Valid`
          (`KismetMaterialLibrary.SetVectorParameterValue` "/Game/Grasslands/Materials/Grass/MP_Foliage_Parameters.MP_Foliage_Parameters" "PlayerPosition" (make `LinearColor` _x _y _z)))
        (:`Is Not Valid`
          _))
      ;[1 0.8941 0.1451] Set VFX direction
      (`/Engine/EditorBlueprintResources/StandardMacros.IsValid` (`|GetArrayItem` (`self.Niagra_VFX_Array_Ref`))
        (:`Is Valid`
          (for _array_element (`self.Niagra_VFX_Array_Ref`)
            (set `self.Niagra_VFX_Ref` _array_element)
            (bind _vector_direction (`/Game/Grasslands/Blueprints/BP_Function_Library.Direction_To_Vector` (`self.Global_Wind_Direction`)))
            (set `self.Vector_Direction` _vector_direction)
            (`NiagaraComponent.SetVariableVec3` (`NiagaraActor.NiagaraComponent` (`self.Niagra_VFX_Ref`)) "Wind Speed" (* (`self.Vector_Direction`) (`self.Niagra_Wind_Speed`)))))
        (:`Is Not Valid`
          _))
      (if (`self.PlayDemoAnimations?`)
        ;[1 1 1] Blueprint Driven Examples - Do Once
        (`/Engine/EditorBlueprintResources/StandardMacros.DoOnce` false
          (:`Completed`
            (`KismetSystemLibrary.Delay` 2.0)
            ;[1 0.944 0.4937] Change Wind Direction Runtime
            ;;[1 1 1] Set Desired New Direction
            (set `self.New_Wind_Direction` 0.85)
            (set `self.New_Direction_Set?` false)
            (set `self.Previous_Wind_Direction` (`self.Global_Wind_Direction`))
            (set `self.Wind_Power_Min_Ref` (`self.Wind_Power_Min`))
            (set `self.Wind_Power_Max_Ref` (`self.Wind_Power_Max`))
            (`KismetSystemLibrary.PrintString` "Update Wind Direction")
            (bind (_direction _new_direction _noise_swap_value) (`Timeline|TL_Change_Wind_Direction`)
              (:`Update`
                (if (>= _new_direction 1.0)
                  (if (not (`self.New_Direction_Set?`))
                    (set `self.New_Direction_Set?` true)
                    (set `self.Global_Wind_Direction` (`self.New_Wind_Direction`))))
                (set `self.Noise_Swap_Value` _noise_swap_value))
              (:`Finished`
                ;[1 0.944 0.4937] Change Wind Direction Runtime
                (`KismetSystemLibrary.Delay` 2.0)
                ;;[1 1 1] Set Desired New Direction
                (set `self.New_Wind_Direction` 0.7)
                (set `self.New_Direction_Set?` false)
                (set `self.Previous_Wind_Direction` (`self.Global_Wind_Direction`))
                (set `self.Wind_Power_Min_Ref` (`self.Wind_Power_Min`))
                (set `self.Wind_Power_Max_Ref` (`self.Wind_Power_Max`))
                (`KismetSystemLibrary.PrintString` "Update Wind Direction")
                (bind (_direction_2 _new_direction_2 _noise_swap_value_2) (`Timeline|TL_Change_Wind_Direction_02`)
                  (:`Update`
                    (if (>= _new_direction_2 1.0)
                      (if (not (`self.New_Direction_Set?`))
                        (set `self.New_Direction_Set?` true)
                        (set `self.Global_Wind_Direction` (`self.New_Wind_Direction`))))
                    (set `self.Noise_Swap_Value` _noise_swap_value_2))
                  (:`Finished`
                    ;[1 0.3804 0.8745] Showcase - Mask Based Height
                    ;;[1 1 1] Pause Time
                    (set `self.Time_Add_Value_Ref` (`self.Time_Add_Value`))
                    (bind (_direction_3 _newtrack_0) (`Timeline|Pause_Time`)
                      (:`Update`
                        (set `self.Time_Add_Value` (`KismetMathLibrary.Lerp` (`self.Time_Add_Value_Ref`) 0.0 _newtrack_0)))
                      (:`Finished`
                        ;;[1 0.3804 0.8745] Mask Power
                        (set `self.Mask_Tiling_Ref` (`self.Mask_Tiling`))
                        (set `self.Mask_Power_Ref` (`self.Mask_Power`))
                        (`KismetSystemLibrary.Delay` 1.0)
                        (`KismetSystemLibrary.PrintString` "Height Mask Power")
                        (bind (_direction_4 _newtrack_0_2) (`Timeline|TL_Mask_Power`)
                          (:`Update`
                            (set `self.Mask_Power` (`KismetMathLibrary.Lerp` (`self.Mask_Power_Ref`) 0.0 _newtrack_0_2)))
                          (:`Finished`
                            (bind (_direction_5 _newtrack_0_3) (`Timeline|TL_Mask_Power_02`)
                              (:`Update`
                                (set `self.Mask_Power` (`KismetMathLibrary.Lerp` _mask_power_ref (* _mask_power_ref 10.0) _newtrack_0_3)))
                              (:`Finished`
                                (set `self.Mask_Power_Ref` (`self.Mask_Power`))
                                ;;[1 0.3804 0.8745] Mask Time Emulate Tiling
                                (set `self.Mask_Time_Ref` (`self.Mask_Time`))
                                (bind (_direction_6 _newtrack_0_4) (`Timeline|TL_Mask_Time`)
                                  (:`Update`
                                    (set `self.Mask_Time` (`KismetMathLibrary.Lerp` 0.0 2.0 _newtrack_0_4)))
                                  (:`Finished`
                                    ;;[1 1 1] Resume Time
                                    (bind (_direction_7 _newtrack_0_5) (`Timeline|Timeline`)
                                      (:`Update`
                                        (set `self.Time_Add_Value` (`KismetMathLibrary.Lerp` 0.0 (`self.Time_Add_Value_Ref`) _newtrack_0_5)))
                                      (:`Finished`
                                        ;[0.3373 0.4118 1] Showcase - Diffuse Noise Color
                                        ;;[0.3373 0.4118 1] Change Noise Color
                                        (set `self.Color_Lower_Ref` (`self.Color_Lower`))
                                        (set `self.Color_Upper_Ref` (`self.Color_Upper`))
                                        (set `self.Color_Noise_Ref` (`self.Color_Noise`))
                                        (`KismetSystemLibrary.Delay` 2.0)
                                        (bind (_direction_8 _newtrack_1) (`Timeline|TL_Noise_Color`)
                                          (:`Update`
                                            (set `self.Color_Noise` _newtrack_1))
                                          (:`Finished`
                                            ;;[0.3373 0.4118 1] Change Color All
                                            (set `self.Color_Lower_Ref` (`self.Color_Lower`))
                                            (set `self.Color_Upper_Ref` (`self.Color_Upper`))
                                            (set `self.Color_Noise_Ref` (`self.Color_Noise`))
                                            (`KismetSystemLibrary.Delay` 2.0)
                                            (bind (_direction_9 _newtrack_1_2) (`Timeline|TL_Change_Color_All_01`)
                                              (:`Update`
                                                (set `self.Color_Lower` (`KismetMathLibrary.LinearColorLerp` (`self.Color_Lower_Ref`) (struct :`R` 0.05098 :`G` 0.082353 :`B` 0.062745 :`A` 1.0) _newtrack_1_2))
                                                (set `self.Color_Upper` (`KismetMathLibrary.LinearColorLerp` (`self.Color_Upper_Ref`) (struct :`R` 0.921569 :`B` 0.066667 :`A` 1.0) _newtrack_1_2))
                                                (set `self.Color_Noise` (`KismetMathLibrary.LinearColorLerp` (`self.Color_Noise_Ref`) (struct :`R` 0.078125 :`G` 0.078125 :`B` 0.075685 :`A` 1.0) _newtrack_1_2)))
                                              (:`Finished`
                                                ;;[0.3373 0.4118 1] Change Color Lower, Upper & Noise
                                                (set `self.Color_Lower_Ref` (`self.Color_Lower`))
                                                (set `self.Color_Upper_Ref` (`self.Color_Upper`))
                                                (set `self.Color_Noise_Ref` (`self.Color_Noise`))
                                                (`KismetSystemLibrary.Delay` 2.0)
                                                (bind (_direction_10 _newtrack_1_3) (`Timeline|TL_Change_Color_Lower`)
                                                  (:`Update`
                                                    (set `self.Color_Lower` (`KismetMathLibrary.LinearColorLerp` (`self.Color_Lower_Ref`) (struct :`R` 0.003922 :`G` 0.003922 :`A` 1.0) _newtrack_1_3)))
                                                  (:`Finished`
                                                    (bind (_direction_11 _newtrack_1_4) (`Timeline|TL_Change_Color_Upper_And_Noise`)
                                                      (:`Update`
                                                        (set `self.Color_Upper` (`KismetMathLibrary.LinearColorLerp` (`self.Color_Upper_Ref`) (struct :`R` 0.011765 :`G` 0.007843 :`A` 1.0) _newtrack_1_4))
                                                        (set `self.Color_Noise` (`KismetMathLibrary.LinearColorLerp` (`self.Color_Noise_Ref`) (struct :`R` 0.086275 :`G` 0.090196 :`B` 0.047059 :`A` 1.0) _newtrack_1_4)))
                                                      (:`Finished`
                                                        ;;[0.3373 0.4118 1] Change Color All 03
                                                        (set `self.Color_Lower_Ref` (`self.Color_Lower`))
                                                        (set `self.Color_Upper_Ref` (`self.Color_Upper`))
                                                        (set `self.Color_Noise_Ref` (`self.Color_Noise`))
                                                        (`KismetSystemLibrary.Delay` 2.0)
                                                        (bind (_direction_12 _newtrack_1_5) (`Timeline|TL_Change_Color_All_03`)
                                                          (:`Update`
                                                            (set `self.Color_Lower` (`KismetMathLibrary.LinearColorLerp` (`self.Color_Lower_Ref`) (struct :`R` 0.066667 :`G` 0.105882 :`B` 0.003922 :`A` 1.0) _newtrack_1_5))
                                                            (set `self.Color_Upper` (`KismetMathLibrary.LinearColorLerp` (`self.Color_Upper_Ref`) (struct :`R` 1.0 :`B` 0.054902 :`A` 1.0) _newtrack_1_5))
                                                            (set `self.Color_Noise` (`KismetMathLibrary.LinearColorLerp` (`self.Color_Noise_Ref`) (struct :`R` 0.141176 :`G` 0.207843 :`B` 0.05098 :`A` 1.0) _newtrack_1_5)))
                                                          (:`Finished`
                                                            ;;[0.3373 0.4118 1] Change to Original Color
                                                            (set `self.Color_Lower_Ref` (`self.Color_Lower`))
                                                            (set `self.Color_Upper_Ref` (`self.Color_Upper`))
                                                            (set `self.Color_Noise_Ref` (`self.Color_Noise`))
                                                            (`KismetSystemLibrary.Delay` 2.0)
                                                            (bind (_direction_13 _newtrack_1_6) (`Timeline|TL_Change_Color_All_04`)
                                                              (:`Update`
                                                                (set `self.Color_Lower` (`KismetMathLibrary.LinearColorLerp` (`self.Color_Lower_Ref`) (struct :`R` 0.031373 :`G` 0.082353 :`A` 1.0) _newtrack_1_6))
                                                                (set `self.Color_Upper` (`KismetMathLibrary.LinearColorLerp` (`self.Color_Upper_Ref`) (struct :`R` 0.035294 :`G` 0.090196 :`A` 1.0) _newtrack_1_6))
                                                                (set `self.Color_Noise` (`KismetMathLibrary.LinearColorLerp` (`self.Color_Noise_Ref`) (struct :`R` 0.058824 :`G` 0.156863 :`B` 0.007843 :`A` 1.0) _newtrack_1_6)))
                                                              (:`Finished`
                                                                ;[0.5686 1 0.4353] Wind Intensity, Gusts & Calm Wind
                                                                ;;[0.5686 1 0.4353] Slow Down Wind & Less Power
                                                                (`KismetSystemLibrary.PrintString` "Calm Wind")
                                                                (set `self.Time_Add_Value_Ref` (`self.Time_Add_Value`))
                                                                (set `self.Wind_Power_Min_Ref` (`self.Wind_Power_Min`))
                                                                (set `self.Wind_Power_Max_Ref` (`self.Wind_Power_Max`))
                                                                (bind (_direction_14 _newtrack_0_6) (`Timeline|TL_Slow_Wind_Low_Power`)
                                                                  (:`Update`
                                                                    (set `self.Time_Add_Value` (`KismetMathLibrary.Lerp` _time_add_value_ref_2 (- _time_add_value_ref_2 0.01) _newtrack_0_6))
                                                                    (set `self.Wind_Power_Max` (`KismetMathLibrary.Lerp` _wind_power_max_ref_2 (/ _wind_power_max_ref_2 2.0) _newtrack_0_6))
                                                                    (set `self.Wind_Power_Min` (`KismetMathLibrary.Lerp` _wind_power_min_ref (/ _wind_power_min_ref 2.0) _newtrack_0_6)))
                                                                  (:`Finished`
                                                                    ;;[0.5686 1 0.4353] Calm Wind
                                                                    (`KismetSystemLibrary.PrintString` "Calm Wind")
                                                                    (bind (_direction_15 _newtrack_0_7) (`Timeline|TL_Calm_Wind`)
                                                                      (:`Update`
                                                                        (set `self.Calm_Wind` (`KismetMathLibrary.Lerp` 0.0 1.0 _newtrack_0_7)))
                                                                      (:`Finished`
                                                                        ;;[0.5686 1 0.4353] Wind Gusts
                                                                        (`KismetSystemLibrary.PrintString` "Wind Gusts")
                                                                        (set `self.Time_Add_Value_Ref` (`self.Time_Add_Value`))
                                                                        (set `self.Wind_Power_Max_Ref` (`self.Wind_Power_Max`))
                                                                        (bind (_direction_16 _newtrack_0_8) (`Timeline|TL_Wind_Gusts`)
                                                                          (:`Update`
                                                                            (bind _returnvalue (`KismetMathLibrary.FClamp` _newtrack_0_8))
                                                                            (set `self.Time_Add_Value` (`KismetMathLibrary.Lerp` _time_add_value_ref (+ _time_add_value_ref 0.015) _returnvalue))
                                                                            (set `self.Wind_Power_Max` (`KismetMathLibrary.Lerp` _wind_power_max_ref (* _wind_power_max_ref 1.3) _returnvalue))))))))))))))))))))))))))))))))))))))))

(fn `UserConstructionScript`)